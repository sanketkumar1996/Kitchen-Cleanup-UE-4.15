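; Plate actor for a VR game that can be picked up, dropped and destroyed for score.
; On BeginPlay it binds DestroyAll to the PlatePopper dispatcher of the first Bp_buttonPopper found.
; DestroyAll passes PlatesDestroyed to MyVRGamemode's TargetScores, then destroys the plate.
; PickUp and DropOff attach and detach the actor, both enabling mesh physics; the drop impulse is zero.
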(event Custom|DestroyAll
  ;[1 1 1] Event Dispatcher - to destroy all plates and update the score
  (bind _asmy_vrgamemode (Utilities|Casting|CastToMyVRGamemode (Game|GetGameMode)))
  (Default|TargetScores _asmy_vrgamemode (Variables|Default|GetplatesDestroyed))
  (Actor|DestroyActor))

(event Collision|EventActorBeginOverlap
  (params (OtherActor :type Actor%20Object%20Reference)))

(event EventBeginPlay
  ;[1 1 1] Event Dispatcher - to destroy all plates and update the score
  (bind _outactors (Actor|GetAllActorsOfClass "/Game/bp_buttonPopper.bp_buttonPopper_C"))
  (bind _output_get (Variables|Default|SetButtonPopper (Utilities|Array|Get(acopy) _outactors)))
  (EventDispatchers|BindEventtoPlatePopper _output_get (delegate Custom|DestroyAll)))

(event EventPickUp
  (params (ActorToAttachTo :type Scene%20Component%20Object%20Reference))
  ;[1 1 1] Pick up plates
  (Physics|SetSimulatePhysics (Variables|Default|Getplates_mesh) true)
  (Transformation|AttachComponentToComponent (VehicleSound|GetRootComponent) ActorToAttachTo "None" "KeepWorld" "KeepWorld" "KeepWorld" true))

(event EventTick
  (params (DeltaSeconds :type Float%20%28single-precision%29)))

(event EventDropOff
  ;[1 1 1] Drop the plates
  (Physics|SetSimulatePhysics (Variables|Default|Getplates_mesh) true)
  (Transformation|DetachFromActor "KeepWorld" "KeepWorld" "KeepWorld")
  (Physics|AddImpulse (Variables|Default|Getplates_mesh) "0.000000,0.000000,0.000000" "None" false))

(fn ConstructionScript)